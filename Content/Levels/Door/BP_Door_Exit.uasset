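; BP_Door_Exit is an exit door that stops the current experiment episode when a PawnMain overlaps its CollisionStopEpisode component.
; The overlap asks GameModeMain to stop the episode through ExperimentStopEpisode.
; If that returns true, the door disables the trigger's collision and sets a timer that restores query-only collision after a few seconds, logging both changes with PrintString.
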(event OnComponentBeginOverlap(CollisionStopEpisode)
  (params (OverlappedComponent :type Primitive%20Component%20Object%20Reference) (OtherActor :type Actor%20Object%20Reference) (OtherComp :type Primitive%20Component%20Object%20Reference) (OtherBodyIndex :type Integer) (bFromSweep :type Boolean) (SweepResult :type Hit%20Result%20Structure%20%28by%20ref%29))
  ;[1 1 1] Stop Episode
  (bind _aspawn_main (Utilities|Casting|CastToPawnMain OtherActor))
  (Utilities|IsValid _aspawn_main
    (:Is%20Valid
      (bind _asgame_mode_main (Utilities|Casting|CastToGameModeMain (Game|GetGameMode)))
      (Utilities|IsValid _asgame_mode_main
        (:Is%20Valid
          (bind _returnvalue (Class|GameModeMain|ExperimentStopEpisode _asgame_mode_main))
          (if _returnvalue
            (CallFunction|DisableCollision)
            (bind _returnvalue_2 (Utilities|Time|SetTimerbyEvent (delegate Custom|EnableCollisions) 5.0))
            (Variables|Default|SetTimerHandleCollisions _returnvalue_2)))))))

(event Custom|EnableCollisions
  ;[1 1 1] Stop Episode
  (CallFunction|EnableCollision))

(fn ConstructionScript
  (|CallParentFunction))

(fn EnableCollision
  (bind _collisionstopepisode (Variables|Default|GetCollisionStopEpisode))
  (Utilities|IsValid _collisionstopepisode
    (:Is%20Valid
      (Collision|SetCollisionEnabled _collisionstopepisode "QueryOnly")
      (Development|PrintString "Exit Door: Enabled Collision"))))

(fn DisableCollision
  (bind _collisionstopepisode (Variables|Default|GetCollisionStopEpisode))
  (Utilities|IsValid _collisionstopepisode
    (:Is%20Valid
      (Collision|SetCollisionEnabled _collisionstopepisode "NoCollision")
      (Development|PrintString "Exit Door: Disabled Collision"))))