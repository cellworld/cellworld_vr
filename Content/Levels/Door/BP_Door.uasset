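; BP_Door is a door that opens when the player pawn (PawnMain) enters its collision volume and closes when it leaves.
; Overlap events play and reverse DoorAnimationTimeline, whose OpenDoor track drives the relative location of DoorMesh.
; StartEpisode is an empty event, and the GameModeMain logic that would start an experiment episode is disconnected, so it never runs.
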(event OnComponentBeginOverlap(CollisionDoor)
  (params (OverlappedComponent :type Primitive%20Component%20Object%20Reference) (OtherActor :type Actor%20Object%20Reference) (OtherComp :type Primitive%20Component%20Object%20Reference) (OtherBodyIndex :type Integer) (bFromSweep :type Boolean) (SweepResult :type Hit%20Result%20Structure%20%28by%20ref%29))
  (Utilities|Casting|CastToPawnMain OtherActor)
  (bind _opendoor (Timeline|DoorAnimationTimeline Play)
    (:Update
      (Transformation|SetRelativeLocation (Variables|Default|GetDoorMesh) _opendoor false false))))

(event OnComponentEndOverlap(CollisionDoor)
  (params (OverlappedComponent :type Primitive%20Component%20Object%20Reference) (OtherActor :type Actor%20Object%20Reference) (OtherComp :type Primitive%20Component%20Object%20Reference) (OtherBodyIndex :type Integer))
  (Utilities|Casting|CastToPawnMain OtherActor)
  (bind _opendoor (Timeline|DoorAnimationTimeline Reverse)
    (:Update
      (Transformation|SetRelativeLocation (Variables|Default|GetDoorMesh) _opendoor false false))))

(event Custom|StartEpisode
  ;[1 1 1] Stop episode when leaving door area
)

(fn ConstructionScript)