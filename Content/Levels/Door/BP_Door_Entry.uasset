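; Entry door Blueprint that starts an experiment episode when its start-episode collision volume is overlapped.
; The overlap casts the game mode to GameModeMain, calls ExperimentStartEpisode if the ExperimentServiceMonitor is valid, and prints the result or an error.
; The overlap does not filter by actor, and the separate door collision only prints a debug greeting.
; The construction script just runs the parent's.
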(event OnComponentBeginOverlap(CollisionDoor)
  (params (OverlappedComponent :type Primitive%20Component%20Object%20Reference) (OtherActor :type Actor%20Object%20Reference) (OtherComp :type Primitive%20Component%20Object%20Reference) (OtherBodyIndex :type Integer) (bFromSweep :type Boolean) (SweepResult :type Hit%20Result%20Structure%20%28by%20ref%29))
  (Development|PrintString "Hello"))

(event OnComponentBeginOverlap(CollisionStartEpisode)
  (params (OverlappedComponent :type Primitive%20Component%20Object%20Reference) (OtherActor :type Actor%20Object%20Reference) (OtherComp :type Primitive%20Component%20Object%20Reference) (OtherBodyIndex :type Integer) (bFromSweep :type Boolean) (SweepResult :type Hit%20Result%20Structure%20%28by%20ref%29))
  ;[1 1 1] Start Episode
  (Development|PrintString "COLLISION: START EPISODE" true true "(R=0.000000,G=0.660000,B=1.000000,A=1.000000)" 1e+01)
  (bind _asgame_mode_main (Utilities|Casting|CastToGameModeMain (Game|GetGameMode)))
  (Utilities|IsValid (Variables|/Script/cellworld_vr.GameModeMain|GetExperimentServiceMonitor _asgame_mode_main)
    (:Is%20Valid
      (bind _returnvalue (Class|GameModeMain|ExperimentStartEpisode _asgame_mode_main))
      (Development|PrintString (Utilities|String|ToString(Boolean) _returnvalue)))
    (:Is%20Not%20Valid
      (Development|PrintString "[BP_DOOR_ENTRY] ExperimentServiceMonitor NOT VALID"))))

(event EventBeginPlay)

(event Collision|EventActorBeginOverlap
  (params (OtherActor :type Actor%20Object%20Reference)))

(event EventTick
  (params (DeltaSeconds :type Float%20%28single-precision%29)))

(fn ConstructionScript
  (|CallParentFunction))