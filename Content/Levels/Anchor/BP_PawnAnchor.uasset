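; VR pawn for the spatial anchor level that lets the right motion controller point at anchor models to hover them.
; In selection mode, Tick sphere-traces from the controller, asking SpatialAnchorManagerComponentAC to update hover highlights on anchor models.
; A two-point spline drives a spline-mesh laser that stretches to the hit or maximum range, collapsing outside selection mode.
; The construction script wires the anchor and menu manager components to their attachment points.
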(event EventTick
  (params (DeltaSeconds :type Float%20%28single-precision%29))
  (bind _spatialanchormanagercomponent_ac (Variables|Default|GetSpatialAnchorManagerComponent_AC))
  (bind _splinecomponent (Variables|Default|GetSplineComponent))
  (bind _motioncontrollerright (Variables|Default|GetMotionControllerRight))
  (bind _splinecomponent_2 (Variables|Default|GetSplineComponent))
  (bind _returnvalue (Transformation|GetWorldLocation _motioncontrollerright))
  (bind _returnvalue_2 (Math|Vector|GetForwardVector _motioncontrollerright))
  (bind _returnvalue_3 (* _returnvalue_2 1e+04))
  (bind _returnvalue_4 (+ _returnvalue _returnvalue_3))
  ;[1 1 1] Hover Anchor
  (if (Variables|/Game/SpatialAnchorsSample/Blueprints/Components/BP_SpatialAnchorManagerComponent.BP_SpatialAnchorManagerComponent_C|GetbSelectionMode _spatialanchormanagercomponent_ac)
    (bind _outhit (Collision|SphereTraceByChannel _returnvalue _returnvalue_4 1.0 "TraceTypeQuery1" false 0 "None" true "(R=1.000000,G=1.000000,B=1.000000,A=1.000000)" "(R=0.000000,G=1.000000,B=0.000000,A=1.000000)" 0.0))
    ;;[1 1 1] Update Laser Pointer length based on hit
    (if (.bblockinghit _outhit)
      (Spline|SetLocationatSplinePoint _splinecomponent_2 1 (.location _outhit) "World" true)
      (else
        (Spline|SetLocationatSplinePoint _splinecomponent_2 1 _returnvalue_4 "World" true)))
    (CallFunction|UpdateSplineMesh)
    ;;[1 1 1] Determining Logic of which anchors to highlight/unhighlight
    (bind _asbp_spatial_anchor_model (Utilities|Casting|CastToBP_SpatialAnchorModel (.hitactor _outhit))
      (:then
        (if (not (== _asbp_spatial_anchor_model (Variables|Default|GetLast%20Hovered%20Anchor)))
          (Default|UnsetHovered _spatialanchormanagercomponent_ac (Variables|Default|GetLast%20Hovered%20Anchor))
          (Default|SetHovered _spatialanchormanagercomponent_ac _asbp_spatial_anchor_model)
          (Variables|Default|SetLast%20Hovered%20Anchor (Variables|Default|GetLast%20Hovered%20Anchor))))
      (:CastFailed
        (Default|UnsetHovered _spatialanchormanagercomponent_ac (Variables|Default|GetLast%20Hovered%20Anchor))
        (Variables|Default|SetLast%20Hovered%20Anchor 0)))
    (else
      ;;[1 1 1] If not in selection mode, hide the laser pointer
      (Spline|SetLocationatSplinePoint _splinecomponent 1 (Spline|GetLocationatSplinePoint _splinecomponent 0 "World") "World" true)
      (CallFunction|UpdateSplineMesh)
      (Development|PrintString "UpdateSplineMesh"))))

(fn ConstructionScript
  (bind _menumanagercomponent_ac (Variables|Default|GetMenuManagerComponent_AC))
  (bind _spatialanchormanagercomponent_ac (Variables|Default|GetSpatialAnchorManagerComponent_AC))
  (Variables|/Game/SpatialAnchorsSample/Blueprints/Components/BP_SpatialAnchorManagerComponent.BP_SpatialAnchorManagerComponent_C|SetModelSpawnPositioner _spatialanchormanagercomponent_ac (Variables|Default|GetModelSpawnPoint))
  (Variables|/Game/SpatialAnchorsSample/Blueprints/Components/BP_MenuManagerComponent.BP_MenuManagerComponent_C|SetSpatialAnchorManager _menumanagercomponent_ac _spatialanchormanagercomponent_ac)
  (Variables|/Game/SpatialAnchorsSample/Blueprints/Components/BP_MenuManagerComponent.BP_MenuManagerComponent_C|SetMainMenuPositioner _menumanagercomponent_ac (Variables|Default|GetMainMenuAttachmentPoint))
  (Variables|/Game/SpatialAnchorsSample/Blueprints/Components/BP_MenuManagerComponent.BP_MenuManagerComponent_C|SetAnchorMenuPositioner _menumanagercomponent_ac (Variables|Default|GetAnchorMenuAttachmentPoint))
  (Development|PrintString "BP_PawnAnchor ConstructionScript Done"))

(fn UpdateSplineMesh
  (bind _splinecomponent (Variables|Default|GetSplineComponent))
  (bind (_location _tangent) (Spline|GetLocationandTangentatSplinePoint _splinecomponent 1 "Local"))
  (bind (_location_2 _tangent_2) (Spline|GetLocationandTangentatSplinePoint _splinecomponent 0 "Local"))
  (SplineMesh|SetStartandEnd (Variables|Default|GetSplineMesh) _location_2 _tangent_2 _location _tangent true :!class /Script/Engine.SplineMeshComponent))