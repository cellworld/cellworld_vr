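; Save game object for the spatial anchors sample that records Oculus spatial anchors as a SavedAnchors array of UUID and local-save flag.
; CreateSaveDatafromAnchors adds only anchors stored locally and prints a failure message for the others.
; MergeSaveData adds unique entries for all given anchors with their current local flag and returns itself.
; SetExistingUUIDs adds unique entries from raw UUIDs, marking each as saved locally.
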(event Custom|Create%20Save%20Data%20from%20Anchors
  (params (Anchors :type Array%20of%20BP%20Spatial%20Anchor%20Model%20Object%20References))
  (for _array_element Anchors
    (if (Class|OculusXRAnchorComponent|IsStoredatLocation (Variables|/Game/SpatialAnchorsSample/Blueprints/BP_SpatialAnchorModel.BP_SpatialAnchorModel_C|GetOculusSpatialAnchor _array_element) "Local")
      (Utilities|Array|Add (Variables|Default|GetSavedAnchors) (Utilities|Struct|MakeStruct_SavedAnchor (Class|OculusXRAnchorComponent|GetUUID (Variables|/Game/SpatialAnchorsSample/Blueprints/BP_SpatialAnchorModel.BP_SpatialAnchorModel_C|GetOculusSpatialAnchor _array_element)) (Class|OculusXRAnchorComponent|IsStoredatLocation (Variables|/Game/SpatialAnchorsSample/Blueprints/BP_SpatialAnchorModel.BP_SpatialAnchorModel_C|GetOculusSpatialAnchor _array_element) "Local")))
      (else
        (Development|PrintString 0 "FAILED - ANCHORSAVEGAME ISSTOREDATLOCATION" true true "(R=1.000000,G=0.067656,B=0.000000,A=1.000000)" 5.0 "2")))))

(fn MergeSaveData
  (params (Anchors :type Array%20of%20BP%20Spatial%20Anchor%20Model%20Object%20References))
  (for _array_element Anchors
    (Utilities|Array|AddUnique (Variables|Default|GetSavedAnchors) (Utilities|Struct|MakeStruct_SavedAnchor (Class|OculusXRAnchorComponent|GetUUID (Variables|/Game/SpatialAnchorsSample/Blueprints/BP_SpatialAnchorModel.BP_SpatialAnchorModel_C|GetOculusSpatialAnchor _array_element)) (Class|OculusXRAnchorComponent|IsStoredatLocation (Variables|/Game/SpatialAnchorsSample/Blueprints/BP_SpatialAnchorModel.BP_SpatialAnchorModel_C|GetOculusSpatialAnchor _array_element) "Local"))))
  (return self))

(fn SetExistingUUIDs
  (params (AnchorUUIDs :type Array%20of%20Oculus%20XRUUID%20Structures))
  (for _array_element AnchorUUIDs
    (Utilities|Array|AddUnique (Variables|Default|GetSavedAnchors) (Utilities|Struct|MakeStruct_SavedAnchor _array_element true))))