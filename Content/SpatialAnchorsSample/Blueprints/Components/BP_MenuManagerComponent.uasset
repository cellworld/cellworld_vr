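; Component for the Spatial Anchors sample that spawns and manages the main and anchor menus, routing navigation and select input to them.
; The main menu spawns at BeginPlay and follows its positioner every Tick.
; Anchor manager save, unsave and select events respawn an attached anchor menu reflecting selection saved state.
; Unselect, or Tick finding no selection, destroys it and returns the active menu context to main.
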(event Custom|Menu%20Selection%20Up
  ;[1 1 1] Menu Navigation
  (Default|MenuSelectionUp (Variables|MenuReference|GetCurrentMenuContext)))

(event Custom|Menu%20Selection%20Down
  ;[1 1 1] Menu Navigation
  (Default|MenuSelectionDown (Variables|MenuReference|GetCurrentMenuContext)))

(event Custom|Deactivate%20Anchor%20Menu
  (bind _anchormenu (Variables|MenuReference|GetAnchorMenu))
  ;[1 1 1] Context functionality
  (Utilities|IsValid _anchormenu
    (:Is%20Valid
      (Actor|DestroyActor _anchormenu))
    (:Is%20Not%20Valid
      _))
  (Variables|MenuReference|SetCurrentMenuContext (Variables|MenuReference|GetMainMenu)))

(event Custom|Activate%20Anchor%20Menu
  ;[1 1 1] Context functionality
  (bind _anchorselected (Default|HasSelectedAnchor (Variables|Default|GetSpatialAnchorManager)))
  (if _anchorselected
    (bind _anchor_menu (CallFunction|ReturnAnchorMenu (Variables|Default|GetAnchorMenuPositioner)))
    (Variables|MenuReference|SetCurrentMenuContext _anchor_menu)))

(event Custom|Select%20Menu%20Item
  ;[1 1 1] Running logic on selected menu item
  (Default|RunSelect (Variables|MenuReference|GetCurrentMenuContext)))

(event Custom|Select%20Anchor%20Menu%20Item
  (bind _anchormenu (Variables|MenuReference|GetAnchorMenu))
  ;[1 1 1] Running logic on selected menu item
  (Utilities|IsValid _anchormenu
    (:Is%20Valid
      (Default|RunSelect _anchormenu))))

(event Custom|Select%20Main%20Menu%20Item
  (bind _mainmenu (Variables|MenuReference|GetMainMenu))
  ;[1 1 1] Running logic on selected menu item
  (Utilities|IsValid _mainmenu
    (:Is%20Valid
      (Default|RunSelect _mainmenu))))

(event EventTick
  (params (DeltaSeconds :type Float%20%28single-precision%29))
  (bind _mainmenu (Variables|MenuReference|GetMainMenu))
  (Utilities|FlowControl|Sequence
    (:then_0
      ;[1 1 1] Update Main Menu position
      (Utilities|IsValid _mainmenu
        (:Is%20Valid
          (Transformation|SetActorTransform _mainmenu (Transformation|GetWorldTransform (Variables|Default|GetMainMenuPositioner))))))
    (:then_1
      ;[1 1 1] Deactivate Anchor Menu if no longer associated with valid Spatial Anchor
      (bind _anchorselected (Default|HasSelectedAnchor (Variables|Default|GetSpatialAnchorManager)))
      (if (not _anchorselected)
        (CallFunction|DeactivateAnchorMenu)))))

(event EventBeginPlay
  (bind _spatialanchormanager (Variables|Default|GetSpatialAnchorManager))
  (Utilities|FlowControl|Sequence
    (:then_0
      ;[1 1 1] Setting up Main Menu
      (bind _returnvalue (Game|SpawnActorfromClass "/Game/SpatialAnchorsSample/Blueprints/UI/BP_Menu_Main.BP_Menu_Main_C" (Transformation|GetWorldTransform (Variables|Default|GetMainMenuPositioner)) "Undefined" "OverrideRootScale" 0 (Variables|Default|GetSpatialAnchorManager) self 0))
      (bind _output_get (Variables|MenuReference|SetMainMenu _returnvalue))
      (Variables|MenuReference|SetCurrentMenuContext _output_get))
    (:then_1
      ;[1 1 1] Bind events for Spatial Anchor Manager Anchor Functionality Calls
      (Utilities|FlowControl|Sequence
        (:then_0
          (EventDispatchers|BindEventtoAnchorSavedDispatch _spatialanchormanager (delegate Custom|Activate%20Anchor%20Menu)))
        (:then_1
          (EventDispatchers|BindEventtoAnchorUnsavedDispatch _spatialanchormanager (delegate Custom|Activate%20Anchor%20Menu)))
        (:then_2
          (EventDispatchers|BindEventtoAnchorSelectedDispatch _spatialanchormanager (delegate Custom|Activate%20Anchor%20Menu)))))
    (:then_2
      (EventDispatchers|BindEventtoAnchorUnselectedDispatch _spatialanchormanager (delegate Custom|Deactivate%20Anchor%20Menu)))))

(fn ReturnAnchorMenu
  (params (SceneComponentToAttachTo :type Scene%20Component%20Object%20Reference))
  (bind _spatialanchormanager (Variables|Default|GetSpatialAnchorManager))
  ;[1 1 1] If there already exists an Anchor Menu, destroy it and reset it with a new Anchor Menu
  (Utilities|IsValid (Variables|MenuReference|GetAnchorMenu)
    (:Is%20Valid
      (Actor|DestroyActor (Variables|MenuReference|GetAnchorMenu)))
    (:Is%20Not%20Valid
      _))
  (bind _returnvalue (Game|SpawnActorfromClass "/Game/SpatialAnchorsSample/Blueprints/UI/BP_Menu_Anchor.BP_Menu_Anchor_C" (Transformation|GetWorldTransform SceneComponentToAttachTo) "Undefined" "OverrideRootScale" 0 (Default|CheckSelection _spatialanchormanager true) (Default|CheckSelection _spatialanchormanager false) (Variables|Default|GetSpatialAnchorManager) self 0))
  (bind _output_get (Variables|MenuReference|SetAnchorMenu _returnvalue))
  (Transformation|AttachComponentToComponent _output_get SceneComponentToAttachTo "None" "SnapToTarget" "SnapToTarget" "SnapToTarget" true)
  (return _returnvalue))